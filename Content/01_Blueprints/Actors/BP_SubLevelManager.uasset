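; BP_SubLevelManager is an actor that swaps between two streamed sublevels, tied to a puzzle ID.
; On BeginPlay it initializes its puzzle owner component with that ID and starts non-blocking, hidden preloads of both sublevels.
; A LoadSubLevel event unloads the first sublevel and makes the second visible; nothing in this graph calls that event.
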(event `self.ReceiveBeginPlay`
  (`/Game/01_Blueprints/Components/Component_PuzzleOwner.Initialize` (`self.Component_PuzzleOwner`) (`self.Puzzle Id`))
  (`GameplayStatics.LoadStreamLevelBySoftObjectPtr` (`self.SubLevel1`))
  (`GameplayStatics.LoadStreamLevelBySoftObjectPtr` (`self.SubLevel2`)))

(event `/Game/01_Blueprints/Interfaces/Interface_Puzzle.LoadSubLevel`
  (`GameplayStatics.UnloadStreamLevelBySoftObjectPtr` (`self.SubLevel1`))
  (`GameplayStatics.LoadStreamLevelBySoftObjectPtr` (`self.SubLevel2`) true))

(fn `UserConstructionScript`)