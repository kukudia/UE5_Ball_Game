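; BP_GravityCenter is an actor that acts as a point attractor, pulling physics objects toward its location.
; Every Tick it loops over its overlapping components and applies a force toward the actor's center to those simulating physics.
; The force has a fixed magnitude regardless of distance and is not mass-independent, so lighter bodies accelerate faster.
; It also prints each applied force vector to the screen as debug output.
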(event `self.ReceiveTick`
  (params (DeltaSeconds :type "Float (single-precision)"))
  (for _array_element (`self.GetOverlappingComponents`)
    (if (`SceneComponent.IsSimulatingPhysics` _array_element "None")
      (bind _returnvalue (* (`KismetMathLibrary.GetDirectionUnitVector` (`SceneComponent.K2_GetComponentLocation` _array_element) (`self.K2_GetActorLocation`)) 100000.0))
      (`PrimitiveComponent.AddForce` _array_element _returnvalue "None" false)
      (`KismetSystemLibrary.PrintString` (`KismetStringLibrary.Conv_VectorToString` _returnvalue) true false (struct :`R` 1.0 :`G` 1.0 :`B` 1.0 :`A` 1.0) 0.0))))

(fn `UserConstructionScript`)