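; Actor that slides its Cube between StartPosition and EndPosition in world space over a set Duration.
; On BeginPlay, IsReverse selects Play or Reverse on a timeline whose updates lerp and print the position.
; Finishing flips IsReverse without restarting the timeline.
; The construction script's AddControlPoints overwrites StartPosition with EndPosition, leaving both lerp endpoints identical.
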(event `self.ReceiveBeginPlay`
  (`TimelineComponent.SetPlayRate` (`self.TimeLine_Push`) (/ 1.0 (`self.Duration`)))
  (if (`self.IsReverse`)
    (bind (_direction _location) (`Timeline|TimeLine_Push` :!label _label)
      (:`Update`
        (bind _returnvalue (`KismetMathLibrary.VLerp` (`self.StartPosition`) (`self.EndPosition`) _location))
        (`SceneComponent.K2_SetWorldLocation` (`self.Cube`) _returnvalue false false)
        (`KismetSystemLibrary.PrintString` (`KismetStringLibrary.Conv_VectorToString` _returnvalue) true true (struct :`G` 0.66 :`B` 1.0 :`A` 1.0) 0.0))
      (:`Finished`
        (set `self.IsReverse` (not (`self.IsReverse`)))))
    (else
      (goto _label :!via `Reverse`))))

(fn `AddControlPoints`
  (set `self.StartPosition` (`self.StartPosition`))
  (set `self.StartPosition` (`self.EndPosition`)))

(fn `UserConstructionScript`
  (`self.AddControlPoints`))