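; Background music actor that fades in a random track from BGMSet on its Audio component at BeginPlay.
; When audio finishes it increments BGMIndex, replaying only when the index reaches the set length and resets, so other finishes start nothing.
; BGMIndex does not select the track.
; The debug print evaluates the random pick separately, so its name can differ from the playing track.
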(event `self.ReceiveBeginPlay`
  (`self.Play`))

(event `self.Audio.OnAudioFinished`
  (bind _result (`/Engine/EditorBlueprintResources/StandardMacros.IncrementInt` (`self.BGMIndex`))
    (:`  `
      (if (>= _result (`KismetArrayLibrary.Array_Length` (`self.BGMSet`)))
        (set `self.BGMIndex` 0)
        (`self.Play`)))))

(fn `Play`
  (bind _audio (`self.Audio`))
  (bind _outitem (`KismetArrayLibrary.Array_Random` (`self.BGMSet`)))
  (`AudioComponent.SetSound` _audio _outitem)
  (`AudioComponent.FadeIn` _audio 1.0 1.0 0.0 "Linear")
  (`AudioComponent.FadeIn` _audio 1.0 1.0 0.0 "Linear")
  (`KismetSystemLibrary.PrintString` (`KismetSystemLibrary.GetDisplayName` _outitem) true true (struct :`G` 0.66 :`B` 1.0 :`A` 1.0) 10.0))

(fn `UserConstructionScript`)