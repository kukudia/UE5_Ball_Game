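; BP_Grid is a puzzle-linked grid door that moves between an open and a closed position.
; BeginPlay initializes its puzzle owner component with a PuzzleId and calls EventCloseDoor.
; OpenDoor and CloseDoor events drive one timeline forward or in reverse, lerping the grid between start and end locations.
; The open and close sound components play on each move, travel with the grid and stop when the timeline finishes.
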(event `self.ReceiveBeginPlay`
  (`/Game/01_Blueprints/Components/Component_PuzzleOwner.Initialize` (`self.Component_PuzzleOwner`) (`self.PuzzleId`))
  (`self.Event CloseDoor`))

(event `Open`
  (`AudioComponent.Play` (`self.GridOpen`) 0.0)
  (bind (_direction _opendoor) (`Timeline|Timeline_Open` :!label _label)
    (:`Update`
      (bind _output_get (set `self.DoorProgress` _opendoor))
      (bind _returnvalue (`KismetMathLibrary.VLerp` (`self.StartLocation`) (`self.EndLocation`) _output_get))
      (`SceneComponent.K2_SetRelativeLocation` (`self.Grid`) _returnvalue false false)
      (`SceneComponent.K2_SetRelativeLocation` (`self.GridOpen`) _returnvalue false false)
      (`SceneComponent.K2_SetRelativeLocation` (`self.GridClose`) _returnvalue false false))
    (:`Finished`
      (`AudioComponent.Stop` (`self.GridOpen`))
      (`AudioComponent.Stop` (`self.GridClose`)))))

(event `Close`
  (`AudioComponent.Play` (`self.GridClose`) 0.0)
  (goto _label :!via `Reverse`))

(event `self.OpenDoor`
  (`self.Open`))

(event `Event CloseDoor`
  (`self.Close`))

(fn `UserConstructionScript`)