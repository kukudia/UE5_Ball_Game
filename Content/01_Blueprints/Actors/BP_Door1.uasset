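; BP_Door1 is a sliding door actor that opens on OpenDoor and closes itself after a short delay.
; A single timeline lerps StaticMesh1's relative location between start and end positions, playing forward to open and in reverse to close.
; The timeline's Finished event toggles IsOpened and, once open, waits before calling Open again to trigger the reverse.
; BeginPlay initializes ComponentPuzzleOwner with the door's PuzzleId.
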(event `self.ReceiveBeginPlay`
  (`/Game/01_Blueprints/Components/Component_PuzzleOwner.Initialize` (`self.Component_PuzzleOwner`) (`self.PuzzleId`)))

(event `Open`
  (if (not (`self.IsOpened`))
    (bind (_direction _opendoor) (`Timeline|Timeline_Open` :!label _label)
      (:`Update`
        (`SceneComponent.K2_SetRelativeLocation` (`self.StaticMesh1`) (`KismetMathLibrary.VLerp` (`self.StartLocation`) (`self.EndLocation`) _opendoor) false false))
      (:`Finished`
        (bind _output_get (set `self.IsOpened` (not (`self.IsOpened`))))
        (if _output_get
          (`KismetSystemLibrary.Delay` 2.0)
          (`self.Open`))))
    (else
      (goto _label :!via `Reverse`))))

(event `/Game/01_Blueprints/Interfaces/Interface_Puzzle.OpenDoor`
  (`self.Open`))

(fn `UserConstructionScript`)