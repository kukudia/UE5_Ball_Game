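; BP_EntranceBlue is a puzzle checkpoint actor that reacts to a BP_Ball entering its trigger box.
; On overlap, a ball whose color matches CheckState triggers the puzzle interaction, which adds the item through ComponentPuzzleItem; other colors play an invalid sound.
; When a ball leaves, it closes the TargetGrid door if CanClose is set.
; The active-state callback is bound but does nothing, and several material and door nodes are disconnected.
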(event `self.ReceiveBeginPlay`
  (bind _component_puzzleitem (`self.Component_PuzzleItem`))
  (`/Game/01_Blueprints/Components/Component_PuzzleItem.Initialize` _component_puzzleitem (`self.PuzzleItemInfo`))
  (add `/Game/01_Blueprints/Components/Component_PuzzleItem.OnActiveStateChanged` _component_puzzleitem (delegate `StateChanged`)))

(event `StateChanged`
  (params (IsActive :type Boolean) (ItemActor :type "Actor Object Reference"))
  (if IsActive
    _))

(event `self.Box.OnComponentBeginOverlap`
  (params (OverlappedComponent :type "PrimitiveComponent Object Reference") (OtherActor :type "Actor Object Reference") (OtherComp :type "PrimitiveComponent Object Reference") (OtherBodyIndex :type Integer) (bFromSweep :type Boolean) (SweepResult :type "HitResult Structure (by ref)"))
  (bind _asbp_ball (cast `/Game/01_Blueprints/BP_Ball` OtherActor))
  (if (== (`/Game/01_Blueprints/BP_Ball.CurrentColor` _asbp_ball) (`self.Check State`))
    (message `/Game/01_Blueprints/Interfaces/Interface_Puzzle.InteractWithPuzzleItem` self)
    (`KismetSystemLibrary.PrintString` "In check point")
    (else
      (`GameplayStatics.PlaySound2D` "/Game/00_Imports/Audio/Invalid.Invalid" 1.0 1.0 0.0 null null))))

(event `self.Box.OnComponentEndOverlap`
  (params (OverlappedComponent :type "PrimitiveComponent Object Reference") (OtherActor :type "Actor Object Reference") (OtherComp :type "PrimitiveComponent Object Reference") (OtherBodyIndex :type Integer))
  (cast `/Game/01_Blueprints/BP_Ball` OtherActor)
  (`KismetSystemLibrary.PrintString` "In check point" true true (struct :`R` 1.0 :`B` 0.010192 :`A` 1.0))
  (if (`self.CanClose`)
    (`/Game/01_Blueprints/Actors/BP_Grid.Event CloseDoor` (`self.TargetGrid`))))

(event `self.InteractWithPuzzleItem`
  (`/Game/01_Blueprints/Components/Component_PuzzleItem.AddItemToPuzzle` (`self.Component_PuzzleItem`)))

(fn `UserConstructionScript`)