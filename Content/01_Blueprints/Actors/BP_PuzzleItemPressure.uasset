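; BP_PuzzleItemPressure is a pressure-triggered puzzle item actor that changes color with its active state.
; It initializes its ComponentPuzzleItem on BeginPlay and binds state changes to a material swap on Cube1.
; Box begin overlap prints a debug string and sends the puzzle interaction message, while end overlap sets an overlapping BP_Ball's InteractedActor to itself.
; A separate custom event adds the item to the puzzle through the component.
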(event `self.ReceiveBeginPlay`
  (bind _component_puzzleitem (`self.Component_PuzzleItem`))
  (`/Game/01_Blueprints/Components/Component_PuzzleItem.Initialize` _component_puzzleitem (`self.PuzzleItemInfo`))
  (add `/Game/01_Blueprints/Components/Component_PuzzleItem.OnActiveStateChanged` _component_puzzleitem (delegate `StateChanged`)))

(event `StateChanged`
  (params (IsActive :type Boolean) (ItemActor :type "Actor Object Reference"))
  (bind _cube1 (`self.Cube1`))
  (if IsActive
    (`PrimitiveComponent.SetMaterial` _cube1 0 "/Game/01_Blueprints/Material_ColorChange.Material_ColorChange")
    (else
      (`PrimitiveComponent.SetMaterial` _cube1 0 "/Game/LevelPrototyping/Materials/MI_DefaultColorway.MI_DefaultColorway"))))

(event `self.Box.OnComponentBeginOverlap`
  (params (OverlappedComponent :type "PrimitiveComponent Object Reference") (OtherActor :type "Actor Object Reference") (OtherComp :type "PrimitiveComponent Object Reference") (OtherBodyIndex :type Integer) (bFromSweep :type Boolean) (SweepResult :type "HitResult Structure (by ref)"))
  (`KismetSystemLibrary.PrintString` "Hello")
  (message `/Game/01_Blueprints/Interfaces/Interface_Puzzle.InteractWithPuzzleItem` self))

(event `self.Box.OnComponentEndOverlap`
  (params (OverlappedComponent :type "PrimitiveComponent Object Reference") (OtherActor :type "Actor Object Reference") (OtherComp :type "PrimitiveComponent Object Reference") (OtherBodyIndex :type Integer))
  (bind _asbp_ball (cast `/Game/01_Blueprints/BP_Ball` OtherActor))
  (set `/Game/01_Blueprints/BP_Ball.InteractedActor` self _asbp_ball))

(event `CustomEvent`
  (`/Game/01_Blueprints/Components/Component_PuzzleItem.AddItemToPuzzle` (`self.Component_PuzzleItem`)))

(fn `UserConstructionScript`)