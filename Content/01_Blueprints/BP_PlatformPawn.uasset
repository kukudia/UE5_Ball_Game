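; BP_PlatformPawn is a player-controlled tilting platform that spawns a BP_Ball at its Arrow component on BeginPlay.
; It adds the default Enhanced Input mapping context, and IA_Move adds speed- and delta-time-scaled roll and pitch to the Scene component, with yaw held at zero.
; Tick continuously eases the Scene back to level with RInterpTo and updates the stored roll and pitch that input builds on.
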(event `self.ReceiveBeginPlay`
  (`EnhancedInputSubsystemInterface.AddMappingContext` (pcsubsystem `EnhancedInputLocalPlayerSubsystem` (`GameplayStatics.GetPlayerController` 0)) "/Game/Input/IMC_Default.IMC_Default" 0 (struct))
  (`|SpawnActorFromClass` "/Game/01_Blueprints/BP_Ball.BP_Ball_C" (`SceneComponent.K2_GetComponentToWorld` (`self.Arrow`)) "Undefined" "MultiplyWithRoot" null null))

(event `self.ReceiveTick`
  (params (DeltaSeconds :type "Float (single-precision)"))
  (bind _returnvalue (`KismetMathLibrary.RInterpTo` (`SceneComponent.RelativeRotation` (`self.Scene`)) (`self.0`) (`GameplayStatics.GetWorldDeltaSeconds`) 1.0))
  (bind _output_get (set `self.CurrentRot` _returnvalue))
  (set `self.CurrentRoll` (.roll _output_get))
  (set `self.CurrentPitch` (.pitch _output_get))
  (`SceneComponent.K2_SetRelativeRotation` (`self.Scene`) _returnvalue false false))

(event `EnhancedInput|/Game/Input/Actions/IA_Move`
  (params (ActionValue :type "Vector2D Structure") (ElapsedSeconds :type "Float (double-precision)") (TriggeredSeconds :type "Float (double-precision)") (InputAction :type "InputAction Object Reference" :default "/Game/Input/Actions/IA_Move.IA_Move"))
  (:`Triggered`
    (set `self.CurrentRoll` (+ (* ActionValue_X (`self.Speed`) (`GameplayStatics.GetWorldDeltaSeconds`)) (`self.CurrentRoll`)))
    (set `self.CurrentPitch` (+ (* -1.0 (`self.Speed`) (`GameplayStatics.GetWorldDeltaSeconds`) ActionValue_Y) (`self.CurrentPitch`)))
    (`SceneComponent.K2_SetRelativeRotation` (`self.Scene`) (`KismetMathLibrary.MakeRotator` (`self.CurrentRoll`) (`self.CurrentPitch`)) false false)))

(fn `UserConstructionScript`)