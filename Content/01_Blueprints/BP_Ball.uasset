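; Player-controlled physics ball with custom gravity, force-based movement, a cable grapple, color-change interaction and respawn below a height limit.
; Hitting a Bridge blends gravity toward the standard direction nearest the inverted surface normal, then realigns the actor and movement frame.
; F triggers a scan and swaps visibility between two streamed level instances.
; Tick drives gravity, rope pull, rotation and debug output; C pickup appears unfinished, with empty release logic.
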(event `self.ReceiveBeginPlay`
  ;[1 1 1] Start
  (`self.LoadStreamingLevelInstance`)
  (set `LevelStreaming.bShouldBeVisible` true (`self.StreamingLevel1`))
  (set `LevelStreaming.bShouldBeVisible` false (`self.StreamingLevel2`))
  (`self.SetRespawnPoint`))

(event `self.ReceiveTick`
  (params (DeltaSeconds :type "Float (single-precision)"))
  ;[1 1 1] Tick
  (`self.UpdateActorRotation`)
  (`self.ApplyGravity`)
  (`self.Debug`)
  (`self.Roap`)
  (`self.Hold`)
  (`self.Respawn`))

(event `EnhancedInput|/Game/Input/Actions/IA_MouseLook`
  (params (ActionValue :type "Vector2D Structure") (ElapsedSeconds :type "Float (double-precision)") (TriggeredSeconds :type "Float (double-precision)") (InputAction :type "InputAction Object Reference" :default "/Game/Input/Actions/IA_MouseLook.IA_MouseLook"))
  (bind _returnvalue (`self.GetControlRotation`))
  ; Look
  (:`Triggered`
    (`SceneComponent.K2_SetRelativeRotation` (`self.SpringArm`) _returnvalue false false)
    (`self.AddControllerPitchInput` ActionValue_Y)
    (`self.AddControllerYawInput` ActionValue_X)
    (bind _output_get (set `self.MoveRot` (`KismetMathLibrary.TransformRotation` (`KismetMathLibrary.MakeTransform` (0.0 0.0 0.0) (`self.SpringRot`)) (`KismetMathLibrary.MakeRotator` 0.0 0.0 (.yaw _returnvalue)))))
    (`KismetSystemLibrary.PrintString` (`KismetStringLibrary.Conv_RotatorToString` _output_get) true true (struct :`R` 0.351533 :`G` 0.450786 :`B` 0.991102 :`A` 1.0) 0.0)))

(event `EnhancedInput|/Game/Input/Actions/IA_Move`
  (params (ActionValue :type "Vector2D Structure") (ElapsedSeconds :type "Float (double-precision)") (TriggeredSeconds :type "Float (double-precision)") (InputAction :type "InputAction Object Reference" :default "/Game/Input/Actions/IA_Move.IA_Move"))
  (bind _moverot (`self.MoveRot`))
  ; Move
  (:`Triggered`
    (`PrimitiveComponent.AddForce` (`self.Ball`) (* ActionValue_X (`KismetMathLibrary.GetRightVector` _moverot) 50000.0) "None" false)
    (`PrimitiveComponent.AddForce` (`self.Ball`) (* ActionValue_Y (`KismetMathLibrary.GetForwardVector` _moverot) 50000.0) "None" false)))

(event `Key|E`
  (params (Key :type "Key Structure"))
  (:`Pressed`
    (bind _changecoloractor (`self.ChangeColorActor`)
      (:`then`
        (`/Game/01_Blueprints/Actors/BP_ChangeColor.ChangeColor` _changecoloractor self))
      (:`else`))))

(event `Key|F`
  (params (Key :type "Key Structure"))
  (bind _streaminglevel1 (`self.StreamingLevel1`))
  (bind _streaminglevel2 (`self.StreamingLevel2`))
  (bind _bp_scanningsystemcomponent (`self.BP_ScanningSystemComponent`))
  (:`Pressed`
    (`GameplayStatics.PlaySound2D` "/Game/00_Imports/Audio/Scan.Scan" 1.0 1.0 0.0 null null)
    (`KismetSystemLibrary.Delay` 0.3)
    (if (`self.Is Streaming Level 1 Visible`)
      (`/Game/ScanningSystem/BP_ScanningSystemComponent.Scan` _bp_scanningsystemcomponent)
      (set `LevelStreaming.bShouldBeVisible` false _streaminglevel1)
      (set `LevelStreaming.bShouldBeVisible` true _streaminglevel2)
      (set `self.Is Streaming Level 1 Visible` false)
      (else
        (`/Game/ScanningSystem/BP_ScanningSystemComponent.Scan1` _bp_scanningsystemcomponent)
        (set `LevelStreaming.bShouldBeVisible` true _streaminglevel1)
        (set `LevelStreaming.bShouldBeVisible` false _streaminglevel2)
        (set `self.Is Streaming Level 1 Visible` true)))))

(event `Key|LeftMouseButton`
  (params (Key :type "Key Structure"))
  (bind _returnvalue (`SceneComponent.K2_GetComponentLocation` (`self.Ball`)))
  (:`Pressed`
    (bind (_outhit _returnvalue_2) (`KismetSystemLibrary.LineTraceSingle` :`Start` _returnvalue :`End` (+ _returnvalue (* (`KismetMathLibrary.GetForwardVector` (`SceneComponent.K2_GetComponentRotation` (`self.Camera`))) 3000.0)) :`TraceChannel` "TraceTypeQuery1" :`DrawDebugType` "ForDuration"))
    (if _returnvalue_2
      (set `self.GrabPoint` (`.ImpactPoint` (`GameplayStatics.BreakHitResult` _outhit)))
      (`SceneComponent.SetVisibility` (`self.Cable`) true false)
      (set `self.IsGrabbing` true)
      (else
        (`GameplayStatics.PlaySound2D` null 1.0 1.0 0.0 null null))))
  (:`Released`
    (`SceneComponent.SetVisibility` (`self.Cable`) false false)
    (set `self.IsGrabbing` false)))

(event `self.ReceiveHit`
  (params (MyComp :type "PrimitiveComponent Object Reference") (Other :type "Actor Object Reference") (OtherComp :type "PrimitiveComponent Object Reference") (bSelfMoved :type Boolean) (HitLocation :type "Vector Structure") (HitNormal :type "Vector Structure") (NormalImpulse :type "Vector Structure") (Hit :type "HitResult Structure (by ref)"))
  (`KismetSystemLibrary.Delay` 0.2)
  (`self.PlayHitSound` HitLocation HitNormal))

(event `Key|C`
  (params (Key :type "Key Structure"))
  (bind _camera (`self.Camera`))
  (bind _returnvalue (`SceneComponent.K2_GetComponentLocation` _camera))
  (:`Pressed`
    (if (not (`self.IsHolding`))
      (bind (_outhit _returnvalue_2) (`KismetSystemLibrary.LineTraceSingle` :`Start` _returnvalue :`End` (+ _returnvalue (* (`KismetMathLibrary.GetForwardVector` (`SceneComponent.K2_GetComponentRotation` _camera)) (`self.HoldDistance`))) :`TraceChannel` "TraceTypeQuery1" :`DrawDebugType` "ForDuration"))
      (if _returnvalue_2
        (bind (_bblockinghit _binitialoverlap _time _distance _location _impactpoint _normal _impactnormal _physmat _hitactor) (`GameplayStatics.BreakHitResult` _outhit))
        (if (`self.ActorHasTag` _hitactor "Grabbable")
          (bind _output_get (set `self.PickupObject` _hitactor))
          (`PrimitiveComponent.SetSimulatePhysics` (`self.GetComponentByClass` _output_get "/Script/Engine.StaticMeshComponent") false)
          (set `self.IsHolding` true)))))
  (:`Released`
    (if (`self.IsHolding`)
      _)))

(event `self.Ball.OnComponentHit`
  (params (HitComponent :type "PrimitiveComponent Object Reference") (OtherActor :type "Actor Object Reference") (OtherComp :type "PrimitiveComponent Object Reference") (NormalImpulse :type "Vector Structure") (Hit :type "HitResult Structure (by ref)"))
  (bind (_actorrot_roll _actorrot_pitch _actorrot_yaw) (`KismetMathLibrary.BreakRotator` (`self.ActorRot`)))
  (bind _returnvalue (`KismetMathLibrary.NegateVector` (`.Normal` (`GameplayStatics.BreakHitResult` Hit))))
  (bind _returnvalue_2 (- (0.0 0.0 0.0) (`self.CustomGravityDirection`)))
  (bind (_returnvalue_roll _returnvalue_pitch _returnvalue_yaw) (`KismetMathLibrary.BreakRotator` (`KismetMathLibrary.Quat_Rotator` (`KismetMathLibrary.Quat_FindBetweenNormals` (`self.LastGravityDirection`) (`self.CustomGravityDirection`)))))
  (cast `/Game/01_Blueprints/Actors/Bridge` OtherActor)
  (set `self.LastGravityDirection` (`self.CustomGravityDirection`))
  (set `self.CustomGravityDirection` _returnvalue)
  ; Linear Rotate
  (set `self.MaxDot` 0.0)
  (for _array_element (`self.StandardDirections`)
    (bind _returnvalue_3 (`KismetMathLibrary.Dot_VectorVector` _returnvalue _array_element))
    (if (> _returnvalue_3 (`self.MaxDot`))
      (set `self.MaxDot` _returnvalue_3)
      (set `self.BestDir` _array_element)))
  (bind (_direction _newtrack_0) (`Timeline|Timeline`)
    (:`Update`
      (bind _output_get (set `self.CustomGravityDirection` (`KismetMathLibrary.VLerp` (`self.CustomGravityDirection`) (`self.BestDir`) _newtrack_0)))
      (`KismetSystemLibrary.PrintString` (`KismetStringLibrary.Conv_VectorToString` _output_get) true true (struct :`R` 1.0 :`G` 0.999691 :`A` 1.0) 0.0)
      (set `self.ActorRot` (`KismetMathLibrary.MakeRotator` (+ _returnvalue_roll _actorrot_roll) (+ _returnvalue_pitch _actorrot_pitch) (+ _returnvalue_yaw _actorrot_yaw))))
    (:`Finished`
      (`KismetSystemLibrary.Delay` 1.0)
      (set `self.SpringRot` (`KismetMathLibrary.MakeRotFromZX` _returnvalue_2 (`KismetMathLibrary.ProjectVectorOnToPlane` (`SceneComponent.GetForwardVector` (`self.SpringArm`)) _returnvalue_2))))))

(fn `ApplyGravity`
  (bind _returnvalue (* (`self.CustomGravityDirection`) (`self.Gravity`)))
  (`PrimitiveComponent.AddForce` (`self.Ball`) _returnvalue "None" false)
  (`KismetSystemLibrary.PrintString` (`KismetStringLibrary.Conv_VectorToString` _returnvalue) true true (struct :`R` 1.0 :`G` 0.999691 :`A` 1.0) 0.0))

(fn `Debug`
  (bind _ball (`self.Ball`))
  (bind _returnvalue (`SceneComponent.K2_GetComponentLocation` _ball))
  (`KismetSystemLibrary.PrintString` (`KismetStringLibrary.Conv_VectorToString` _returnvalue) true true (struct :`G` 0.66 :`B` 1.0 :`A` 1.0) 0.0)
  (`KismetSystemLibrary.DrawDebugLine` _returnvalue (+ _returnvalue (`SceneComponent.GetComponentVelocity` _ball)) (struct :`R` 0.001258 :`G` 0.140026 :`B` 1.0 :`A` 1.0))
  (`KismetSystemLibrary.DrawDebugLine` _returnvalue (+ _returnvalue (* (`self.CustomGravityDirection`) 100.0)) (struct :`A` 1.0)))

(fn `Hold`
  (bind _camera (`self.Camera`))
  (bind _returnvalue (+ (`SceneComponent.K2_GetComponentLocation` _camera) (* (`KismetMathLibrary.GetForwardVector` (`SceneComponent.K2_GetComponentRotation` _camera)) (`self.HoldDistance`))))
  (`self.PickupObject`
    (:`then`
      (`self.K2_SetActorLocation` _returnvalue)
      (`KismetSystemLibrary.PrintString` (`KismetStringLibrary.Conv_VectorToString` _returnvalue) true true (struct :`G` 0.66 :`B` 1.0 :`A` 1.0) 0.0))
    (:`else`)))

(fn `LoadStreamingLevelInstance`
  (bind (_boutsuccess _returnvalue) (`LevelStreamingDynamic.LoadLevelInstanceBySoftObjectPtr` "/Game/02_Maps/StreamingLevel1.StreamingLevel1" (0.0 0.0 0.0) (struct) "" "/Script/Engine.LevelStreamingDynamic"))
  (set `self.StreamingLevel1` _returnvalue)
  (bind (_boutsuccess_2 _returnvalue_2) (`LevelStreamingDynamic.LoadLevelInstanceBySoftObjectPtr` "/Game/02_Maps/StreamingLevel2.StreamingLevel2" (0.0 0.0 0.0) (struct) "" "/Script/Engine.LevelStreamingDynamic"))
  (set `self.StreamingLevel2` _returnvalue_2))

(fn `PlayHitSound`
  (params (Location :type "Vector Structure") (Strength :type "Vector Structure"))
  (bind _returnvalue (`self.GetVelocity`))
  (bind _returnvalue_2 (* (`KismetMathLibrary.Dot_VectorVector` Strength _returnvalue) (`KismetMathLibrary.VSize` _returnvalue)))
  (if (> _returnvalue_2 5000.0)
    (`GameplayStatics.PlaySoundAtLocation` "/Game/00_Imports/Audio/Hit.Hit" Location (struct) (`KismetMathLibrary.FMin` (/ _returnvalue_2 20000.0) 2.0) 1.0 0.0 null null null null)))

(fn `Respawn`
  (bind (_returnvalue_x _returnvalue_y _returnvalue_z) (`KismetMathLibrary.BreakVector` (`SceneComponent.K2_GetComponentLocation` (`self.Ball`))))
  (if (< _returnvalue_z -2000.0)
    (`PrimitiveComponent.SetPhysicsLinearVelocity` (`self.Ball`) (0.0 0.0 0.0) false "None")
    (`SceneComponent.K2_SetWorldTransform` (`self.Ball`) (`self.RespawnPoint`) false false)))

(fn `Roap`
  (bind _cable (`self.Cable`))
  (if (`self.IsGrabbing`)
    (set `CableComponent.EndLocation` (`KismetMathLibrary.InverseTransformLocation` (`self.GetTransform`) (`self.GrabPoint`)) _cable)
    (`PrimitiveComponent.AddForce` (`self.Ball`) (* (/ 10000000.0 (`CableComponent.CableLength` _cable)) (`KismetMathLibrary.GetDirectionUnitVector` (`self.K2_GetActorLocation`) (`self.GrabPoint`))) "None" false)
    (`PrimitiveComponent.AddForce` (`self.Ball`) (0.0 0.0 50000.0) "None" false)))

(fn `SetRespawnPoint`
  (locals (Print1 :type String :default "Set new respawn point: "))
  (bind _returnvalue (`SceneComponent.K2_GetComponentToWorld` (`self.Ball`)))
  (set `self.RespawnPoint` _returnvalue)
  (`KismetSystemLibrary.PrintString` (`KismetStringLibrary.Concat_StrStr` (`local.Print1`) (`KismetStringLibrary.Conv_TransformToString` _returnvalue))))

(fn `UpdateActorRotation`
  (bind _springrot (`self.SpringRot`))
  (`self.K2_SetActorRotation` _springrot)
  (`KismetSystemLibrary.PrintString` (`KismetStringLibrary.Conv_RotatorToString` _springrot) true true (struct :`R` 0.351533 :`G` 0.450786 :`B` 0.991102 :`A` 1.0) 0.0))

(fn `UserConstructionScript`)