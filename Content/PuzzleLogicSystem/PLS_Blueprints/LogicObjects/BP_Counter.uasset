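; BP_Counter is a puzzle logic object that counts Activate and Deactivate states and signals linked actors when the count crosses a required threshold.
; Reaching the requirement activates linked actors and can disable the counter; dropping just below deactivates them, with optional counting beyond the requirement.
; When visible in game, text renders show the count and a timer-reset material flashes the cube green or red on each crossing.
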(event `self.ReceiveBeginPlay`
  ;[1 1 1] Set text renders
  (`parent.ReceiveBeginPlay`)
  (`self.SetCurrentCounterText` (`self.CurrentCounter`)))

(event `self.OnEnterState`
  (params (State :type "/Game/PuzzleLogicSystem/PLS_Blueprints/Misc/ENUM_LogicTriggerStates Enum" :default "NewEnumerator0"))
  ;[1 1 1] Puzzle logic event received to increase / decrease count.
  (`parent.OnEnterState` State)
  (switch `/Game/PuzzleLogicSystem/PLS_Blueprints/Misc/ENUM_LogicTriggerStates` State
    (:`NewEnumerator0`
      (`self.IncrementCounter`))
    (:`NewEnumerator1`
      (`self.DecrementCounter`))))

(event `ResetCubeMaterial`
  ;[1 1 1] Reset cube material after activation "flash"
  (`PrimitiveComponent.SetMaterial` (`self.LogicCube`) 0 "/Game/PuzzleLogicSystem/Materials/M_LogicCounter.M_LogicCounter"))

(fn `DecrementCounter`
  ;[1 1 1] Decrease count.
  ; Trigger linked actors to deactivate if the current count has just dropped below the required count.
  (if (> (`self.CurrentCounter`) 0)
    (`/Engine/EditorBlueprintResources/StandardMacros.DecrementInt` (`self.CurrentCounter`)
      (:`  `
        (`|ExecutionSequence`
          (:`then_0`
            (if (== (`self.CurrentCounter`) (- (`self.CountRequired`) 1))
              (`self.TriggerLinkedActors` "NewEnumerator1")
              (`self.SetStateChangeMaterial` false)))
          (:`then_1`
            (if (`self.VisibleInGame`)
              (`self.SetCurrentCounterText` (`self.CurrentCounter`)))))))))

(fn `IncrementCounter`
  ;[1 1 1] Increase count.
  ; Trigger linked actors to activate if the required count is reached.
  (if (or (< (`self.CurrentCounter`) (`self.CountRequired`)) (`self.CanCountBeyondRequired`))
    (`/Engine/EditorBlueprintResources/StandardMacros.IncrementInt` (`self.CurrentCounter`)
      (:`  `
        (`|ExecutionSequence`
          (:`then_0`
            (if (== (`self.CurrentCounter`) (`self.CountRequired`))
              (`self.TriggerLinkedActors` "NewEnumerator0")
              (`self.SetStateChangeMaterial` true)
              (if (`self.DisableOnceActivated`)
                (set `self.IsDisabled` true))))
          (:`then_1`
            (if (`self.VisibleInGame`)
              (`self.SetCurrentCounterText` (`self.CurrentCounter`)))))))))

(fn `SetCurrentCounterText`
  (params (Value :type Integer))
  ;[1 1 1] Set text renders to show the current count.
  (`TextRenderComponent.K2_SetText` (`self.TextRender_Value1`) (`KismetTextLibrary.Conv_StringToText` (`KismetStringLibrary.Conv_IntToString` Value)))
  (`TextRenderComponent.K2_SetText` (`self.TextRender_Value2`) (`KismetTextLibrary.Conv_StringToText` (`KismetStringLibrary.Conv_IntToString` Value)))
  (`TextRenderComponent.K2_SetText` (`self.TextRender_Value3`) (`KismetTextLibrary.Conv_StringToText` (`KismetStringLibrary.Conv_IntToString` Value)))
  (`TextRenderComponent.K2_SetText` (`self.TextRender_Value4`) (`KismetTextLibrary.Conv_StringToText` (`KismetStringLibrary.Conv_IntToString` Value))))

(fn `SetStateChangeMaterial`
  (params (IsActivated :type Boolean))
  (bind _logiccube (`self.LogicCube`))
  (bind _timerhandle (`self.TimerHandle`))
  ;[1 1 1] Make the cube "flash" (flash green when just activated, and flash red when just deactivated).
  (if (`self.VisibleInGame`)
    (if (`KismetSystemLibrary.K2_IsValidTimerHandle` _timerhandle)
      (`KismetSystemLibrary.K2_ClearAndInvalidateTimerHandle` _timerhandle))
    (bind _returnvalue (`KismetSystemLibrary.K2_SetTimerDelegate` (`|CreateDelegate` :!event `ResetCubeMaterial`) 0.25))
    (set `self.TimerHandle` _returnvalue)
    (if IsActivated
      (`PrimitiveComponent.SetMaterial` _logiccube 0 "/Game/PuzzleLogicSystem/Materials/M_LogicActivated.M_LogicActivated")
      (else
        (`PrimitiveComponent.SetMaterial` _logiccube 0 "/Game/PuzzleLogicSystem/Materials/M_LogicDeactivated.M_LogicDeactivated")))))

(fn `UserConstructionScript`
  (bind _countrequired (`self.CountRequired`))
  ;[1 1 1] Set text render to show the count required to activate
  (`parent.UserConstructionScript`)
  (`self.SetCurrentCounterText` _countrequired)
  (`TextRenderComponent.K2_SetText` (`self.TextRender_Req`) (`KismetTextLibrary.Conv_IntToText` _countrequired)))