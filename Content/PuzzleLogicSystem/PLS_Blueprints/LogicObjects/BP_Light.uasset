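; Puzzle logic light that switches on or off when it receives a state event.
; Activate and Deactivate call TurnOn or TurnOff and pass the state on to linked actors, while Flip Flop picks one from the point light's visibility.
; TurnOn and TurnOff toggle that visibility and drive color and emissive on a dynamic material instance of the light mesh.
; The construction script applies the light settings and StartOn state in the editor.
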(event `self.OnEnterState`
  (params (State :type "/Game/PuzzleLogicSystem/PLS_Blueprints/Misc/ENUM_LogicTriggerStates Enum" :default "NewEnumerator0"))
  ;[1 1 1] Puzzle logic event received to turn the light on or off, and triggers linked actors.
  (`parent.OnEnterState` State)
  (switch `/Game/PuzzleLogicSystem/PLS_Blueprints/Misc/ENUM_LogicTriggerStates` State
    (:`NewEnumerator0`
      (`self.TurnOn` :!label _label)
      (`self.TriggerLinkedActors` "NewEnumerator0"))
    (:`NewEnumerator1`
      (`self.TurnOff` :!label _label_2)
      (`self.TriggerLinkedActors` "NewEnumerator1"))
    (:`NewEnumerator15`
      (if (`SceneComponent.bVisible` (`self.PointLight`))
        (goto _label_2)
        (else
          (goto _label))))))

(fn `TurnOff`
  ;[1 1 1] Turn the light off, and set the emissive parameter on the light mesh material to be very low.
  (`MaterialInstanceDynamic.SetVectorParameterValue` (`self.LightMeshMaterial`) "LightColor" (`self.OffColor`))
  (`MaterialInstanceDynamic.SetScalarParameterValue` (`self.LightMeshMaterial`) "Emissive" 0.05)
  (`SceneComponent.SetVisibility` (`self.PointLight`) false false))

(fn `TurnOn`
  ;[1 1 1] Turn the light on, and set the material on the light mesh to be very bright/emissive.
  (`MaterialInstanceDynamic.SetVectorParameterValue` (`self.LightMeshMaterial`) "LightColor" (`self.LightColor`))
  (`MaterialInstanceDynamic.SetScalarParameterValue` (`self.LightMeshMaterial`) "Emissive" 10.0)
  (`SceneComponent.SetVisibility` (`self.PointLight`) true false))

(fn `UserConstructionScript`
  (bind _pointlight (`self.PointLight`))
  ;[1 1 1] Sets the light to on of off, and sets the color of the light in the editor.
  (`parent.UserConstructionScript`)
  (`|ExecutionSequence`
    (:`then_0`
      (`LightComponent.SetLightColor` _pointlight (`self.LightColor`) true)
      (`LocalLightComponent.SetIntensityUnits` _pointlight "Unitless")
      (`LightComponent.SetIntensity` _pointlight (`self.Intensity`))
      (`LocalLightComponent.SetAttenuationRadius` _pointlight (`self.Attenuation`))
      (`SceneComponent.SetVisibility` _pointlight true false))
    (:`then_1`
      (bind _returnvalue (`PrimitiveComponent.CreateDynamicMaterialInstance` (`self.LightMesh`) 1 "/Game/PuzzleLogicSystem/Materials/M_Light.M_Light" "None"))
      (bind _output_get (set `self.LightMeshMaterial` _returnvalue))
      (`PrimitiveComponent.SetMaterial` (`self.LightMesh`) 1 _output_get)
      (if (`self.StartOn`)
        (`self.TurnOn`)
        (else
          (`self.TurnOff`))))))