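; BP_Timer is a puzzle logic object that counts down from a set time and sends Activate to its linked actors at zero.
; Incoming logic states start, pause or reset it, and it can auto-start on BeginPlay.
; Tick drives the countdown, then on completion either resets it or disables it.
; When visible in game, text renders show the remaining time and the cube briefly flashes an activated material.
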(event `self.ReceiveBeginPlay`
  ;[1 1 1] Auto activates this timer if set to do so.
  (`parent.ReceiveBeginPlay`)
  (set `self.TimerActive` (`self.AutoStart`)))

(event `self.OnEnterState`
  (params (State :type "/Game/PuzzleLogicSystem/PLS_Blueprints/Misc/ENUM_LogicTriggerStates Enum" :default "NewEnumerator0"))
  ;[1 1 1] Puzzle logic event received to activate the timer, deactivate the timer (stop countdown and reset) or pause the timer.
  (`parent.OnEnterState` State)
  (switch `/Game/PuzzleLogicSystem/PLS_Blueprints/Misc/ENUM_LogicTriggerStates` State
    (:`NewEnumerator0`
      (set `self.TimerActive` true))
    (:`NewEnumerator1`
      (set `self.TimerActive` false)
      (set `self.CurrentTime` (`self.Time`))
      (if (`self.VisibleInGame`)
        (`self.SetCurrentTimerText` (`self.CurrentTime`))))
    (:`NewEnumerator14`
      (set `self.TimerActive` false :!label _label))
    (:`NewEnumerator16`
      (goto _label))))

(event `self.ReceiveTick`
  (params (DeltaSeconds :type "Float (single-precision)"))
  (bind _timerhandle (`self.TimerHandle`))
  ;[1 1 1] Update countdown timer and trigger linked objects when timer reaches 0.
  (`parent.ReceiveTick` DeltaSeconds)
  (if (`self.TimerActive`)
    (set `self.CurrentTime` (- (`self.CurrentTime`) DeltaSeconds))
    (`|ExecutionSequence`
      (:`then_0`
        (if (<= (`self.CurrentTime`) 0.0)
          (set `self.TimerActive` false)
          (if (`self.ResetOnComplete`)
            (set `self.CurrentTime` (`self.Time`))
            (else
              (set `self.CurrentTime` 0.0)
              (set `self.IsDisabled` true)))
          (`self.TriggerLinkedActors` "NewEnumerator0")
          (if (`self.VisibleInGame`)
            (if (`KismetSystemLibrary.K2_IsValidTimerHandle` _timerhandle)
              (`KismetSystemLibrary.K2_ClearAndInvalidateTimerHandle` _timerhandle))
            (bind _returnvalue (`KismetSystemLibrary.K2_SetTimerDelegate` (delegate `ResetCubeMaterial`) 0.25))
            (set `self.TimerHandle` _returnvalue)
            (`PrimitiveComponent.SetMaterial` (`self.LogicCube`) 0 "/Game/PuzzleLogicSystem/Materials/M_LogicActivated.M_LogicActivated"))))
      (:`then_1`
        (if (`self.VisibleInGame`)
          (`self.SetCurrentTimerText` (`self.CurrentTime`)))))))

(event `ResetCubeMaterial`
  ;[1 1 1] Update countdown timer and trigger linked objects when timer reaches 0.
  (`PrimitiveComponent.SetMaterial` (`self.LogicCube`) 0 "/Game/PuzzleLogicSystem/Materials/M_LogicTimer.M_LogicTimer"))

(fn `GetCurrentTimeFormatted`
  (params (Value :type "Float (double-precision)"))
  (returns (OutValue :type Text))
  ;[1 1 1] Returns the timer float variable in a neater format with 1 decimal place.
  (return (`KismetTextLibrary.Conv_DoubleToText` Value "HalfToEven" false true 1 324 1 1)))

(fn `SetCurrentTimerText`
  (params (Value :type "Float (double-precision)"))
  ;[1 1 1] Updates text render to display countdown timer remaining.
  (`TextRenderComponent.K2_SetText` (`self.TextRender_Value1`) (`self.GetCurrentTimeFormatted` Value))
  (`TextRenderComponent.K2_SetText` (`self.TextRender_Value2`) (`self.GetCurrentTimeFormatted` Value))
  (`TextRenderComponent.K2_SetText` (`self.TextRender_Value3`) (`self.GetCurrentTimeFormatted` Value))
  (`TextRenderComponent.K2_SetText` (`self.TextRender_Value4`) (`self.GetCurrentTimeFormatted` Value)))

(fn `UserConstructionScript`
  ;[1 1 1] Set the text render to display the desired countdown time.
  (`parent.UserConstructionScript`)
  (bind _output_get (set `self.CurrentTime` (`self.Time`)))
  (`self.SetCurrentTimerText` _output_get)
  (`TextRenderComponent.K2_SetText` (`self.TextRender_Req`) (`KismetTextLibrary.Conv_DoubleToText` (`self.Time`) "HalfToEven" false true 1 324 1)))