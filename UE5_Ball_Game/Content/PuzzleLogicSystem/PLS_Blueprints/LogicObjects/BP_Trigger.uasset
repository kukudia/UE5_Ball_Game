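; BP_Trigger is a puzzle logic trigger volume that activates or deactivates linked actors when valid actors enter or exit it.
; Overlaps pass a class filter, including child classes, before requesting a state change, which OnEnterState forwards to linked actors.
; Collision toggles for start state, interactability changes and optional one-time activation.
; The construction script sizes the box and visual helper from Size, lifting the box by half its height.
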(event `self.ReceiveBeginPlay`
  (bind _collisionbox (`self.CollisionBox`))
  ;[1 1 1] Toggles collision depending on whether the trigger is active on game start.
  (`parent.ReceiveBeginPlay`)
  (if (`self.TriggerableOnStart`)
    (`PrimitiveComponent.SetCollisionEnabled` _collisionbox "QueryOnly")
    (else
      (`PrimitiveComponent.SetCollisionEnabled` _collisionbox "NoCollision"))))

(event `self.CollisionBox.OnComponentBeginOverlap`
  (params (OverlappedComponent :type "PrimitiveComponent Object Reference") (OtherActor :type "Actor Object Reference") (OtherComp :type "PrimitiveComponent Object Reference") (OtherBodyIndex :type Integer) (bFromSweep :type Boolean) (SweepResult :type "HitResult Structure (by ref)"))
  ;[1 1 1] Attempt to trigger linked actors to activate when valid actors enter this trigger volume.
  ; By default, only PAWN actors trigger entry.
  (if (`self.IsValidActor` OtherActor)
    (`self.AttemptEnterState` "NewEnumerator0")))

(event `self.CollisionBox.OnComponentEndOverlap`
  (params (OverlappedComponent :type "PrimitiveComponent Object Reference") (OtherActor :type "Actor Object Reference") (OtherComp :type "PrimitiveComponent Object Reference") (OtherBodyIndex :type Integer))
  ;[1 1 1] Attempt to trigger linked to deactivate actors when valid actors exit this trigger volume.
  ; By default, only PAWN actors trigger exit.
  (if (`self.IsValidActor` OtherActor)
    (`self.AttemptEnterState` "NewEnumerator1")))

(event `self.OnEnterState`
  (params (State :type "/Game/PuzzleLogicSystem/PLS_Blueprints/Misc/ENUM_LogicTriggerStates Enum" :default "NewEnumerator0"))
  (bind _collisionbox (`self.CollisionBox`))
  ;[1 1 1] Puzzle logic event received to trigger linked actors to activate / deactivate.
  (`parent.OnEnterState` State)
  (switch `/Game/PuzzleLogicSystem/PLS_Blueprints/Misc/ENUM_LogicTriggerStates` State
    (:`NewEnumerator0`
      (`self.TriggerLinkedActors` "NewEnumerator0")
      (`self.CheckActivateOnceOnly`))
    (:`NewEnumerator1`
      (`self.TriggerLinkedActors` "NewEnumerator1"))
    (:`NewEnumerator12`
      (`PrimitiveComponent.SetCollisionEnabled` _collisionbox "QueryOnly"))
    (:`NewEnumerator13`
      (`PrimitiveComponent.SetCollisionEnabled` _collisionbox "NoCollision"))))

(fn `CheckActivateOnceOnly`
  ;[1 1 1] If this trigger is set to only activate once, then disable its collision so it can no longer activate.
  (if (`self.ActivateOnceOnly`)
    (set `self.IsDisabled` true)
    (`PrimitiveComponent.SetCollisionEnabled` (`self.CollisionBox`) "NoCollision")))

(fn `IsValidActor`
  (params (Actor :type "Actor Object Reference"))
  (returns (Valid :type Boolean))
  (locals (ValidClass :type Boolean))
  (bind _returnvalue (`GameplayStatics.GetObjectClass` Actor))
  ;[1 1 1] Checks if the actor that entered this trigger is on the valid actors list. By default, only PAWN actors are accepted.
  (for _array_element (`self.ValidTriggerActors`)
    (if (or (== _array_element _returnvalue) (`KismetMathLibrary.ClassIsChildOf` _returnvalue _array_element))
      (set `local.ValidClass` true)
      (break)))
  (return (`local.ValidClass`)))

(fn `UserConstructionScript`
  (bind _size (`self.Size`))
  ;[1 1 1] Update the trigger volume visual helper size. This is only visible in editor, not in runtime (unless overriden to do so).
  (`parent.UserConstructionScript`)
  (`SceneComponent.SetWorldScale3D` (`self.TriggerVisual`) (/ (`self.Size`) 100.0))
  (`BoxComponent.SetBoxExtent` (`self.CollisionBox`) (* _size 0.5) true)
  (`SceneComponent.K2_SetRelativeLocation` (`self.CollisionBox`) (`KismetMathLibrary.MakeVector` 0.0 0.0 (* (.z _size) 0.5)) false false))