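; Parent Blueprint for puzzle logic objects, which change state and trigger linked actors in a puzzle system.
; AttemptEnterState runs OnEnterState, meant for child overrides, only if CheckCanEnterState passes, which by default blocks disabled objects.
; TriggerLinkedActors maps each state to an array of links, sending each target its configured state through BPI_PuzzleLogic.
; The construction script applies in-game visibility and refreshes the BP_PuzzleLogicVisualiser debug connections.
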(event `self.AttemptEnterState`
  (params (State :type "/Game/PuzzleLogicSystem/PLS_Blueprints/Misc/ENUM_LogicTriggerStates Enum" :default "NewEnumerator0"))
  ;[1 1 1] SHOULD BE CALLED AS A FUNCTION BY CHILDREN BUT NOT IMPLEMENTED/OVERRIDEN
  ; Checks to see if the specific state can be entered.
  (if (`self.CheckCanEnterState` State)
    (`self.OnEnterState` State)))

(event `self.OnEnterState`
  (params (State :type "/Game/PuzzleLogicSystem/PLS_Blueprints/Misc/ENUM_LogicTriggerStates Enum" :default "NewEnumerator0"))
  ;[1 1 1] SHOULD BE IMPLEMENTED/OVERRIDEN BY CHILDREN BUT NOT CALLED AS A FUNCTION
  ; This is the main event that is called by and implemented by most child actors.
  (switch `/Game/PuzzleLogicSystem/PLS_Blueprints/Misc/ENUM_LogicTriggerStates` State
    (:`NewEnumerator16`
      (set `self.IsDisabled` true))))

(event `self.TriggerLinkedActors`
  (params (State :type "/Game/PuzzleLogicSystem/PLS_Blueprints/Misc/ENUM_LogicTriggerStates Enum" :default "NewEnumerator0"))
  ;[1 1 1] SHOULD BE CALLED AS A FUNCTION BY CHILDREN BUT NOT IMPLEMENTED/OVERRIDEN
  ; This function kicks off logic for all linked actors.
  (switch `/Game/PuzzleLogicSystem/PLS_Blueprints/Misc/ENUM_LogicTriggerStates` State
    (:`NewEnumerator0`
      (`self.ActivateActors` (`self.OnActivated`)))
    (:`NewEnumerator1`
      (`self.ActivateActors` (`self.OnDeactivated`)))
    (:`NewEnumerator14`
      (`self.ActivateActors` (`self.OnPaused`)))
    (:`NewEnumerator2`
      (`self.ActivateActors` (`self.OnState1`)))
    (:`NewEnumerator3`
      (`self.ActivateActors` (`self.OnState2`)))
    (:`NewEnumerator4`
      (`self.ActivateActors` (`self.OnState3`)))
    (:`NewEnumerator5`
      (`self.ActivateActors` (`self.OnState4`)))
    (:`NewEnumerator6`
      (`self.ActivateActors` (`self.OnState5`)))
    (:`NewEnumerator12`
      (`self.ActivateActors` (`self.OnInteractable`)))
    (:`NewEnumerator13`
      (`self.ActivateActors` (`self.OnUninteractable`)))
    (:`NewEnumerator16`
      (`self.ActivateActors` (`self.OnDisabled`)))))

(fn `ActivateActors`
  (params (ActorsToTrigger :type "Array of /Game/PuzzleLogicSystem/PLS_Blueprints/Misc/STRUCT_LogicTriggerActor Structure"))
  (locals (ActorToTrigger_Local :type "Actor Object Reference") (TriggerState_Local :type "/Game/PuzzleLogicSystem/PLS_Blueprints/Misc/ENUM_LogicTriggerStates Enum"))
  ;[1 1 1] Triggers actors that are linked to this actors state changes.
  (for _array_element ActorsToTrigger
    (bind (_actortotrigger _triggerstate) (break `/Game/PuzzleLogicSystem/PLS_Blueprints/Misc/STRUCT_LogicTriggerActor` _array_element))
    (bind _output_get (set `local.ActorToTrigger_Local` _actortotrigger))
    (`/Engine/EditorBlueprintResources/StandardMacros.IsValid` _output_get
      (:`Is Valid`
        (set `local.TriggerState_Local` _triggerstate)
        (if (`KismetSystemLibrary.DoesImplementInterface` _output_get "/Game/PuzzleLogicSystem/PLS_Blueprints/Misc/BPI_PuzzleLogic.BPI_PuzzleLogic_C")
          ;[1 1 1] Trigger actor if valid
          (message `/Game/PuzzleLogicSystem/PLS_Blueprints/Misc/BPI_PuzzleLogic.AttemptEnterState` (`local.ActorToTrigger_Local`) (`local.TriggerState_Local`)))))))

(fn `CheckCanEnterState`
  (params (State :type "/Game/PuzzleLogicSystem/PLS_Blueprints/Misc/ENUM_LogicTriggerStates Enum" :default "NewEnumerator0"))
  (returns (Pass :type Boolean))
  ;[1 1 1] By default, ALL states can be entered unless this object has been explicitly disabled.
  ; This check can be overriden by child.
  (return (not (`self.IsDisabled`))))

(fn `InitialiseAdditionalWidgets`
  ;[1 1 1] Called and implemented by child blueprints oto add additional widgets.
)

(fn `IsClassOrChildClass`
  (params (Actor :type "Actor Object Reference") (Class :type "Actor Class Reference"))
  (returns (Valid :type Boolean))
  (bind _returnvalue (`GameplayStatics.GetObjectClass` Actor))
  ;[1 1 1] Checks if the actor is of a specified type (or child of a specified type).
  (return (or (== _returnvalue Class) (`KismetMathLibrary.ClassIsChildOf` _returnvalue Class))))

(fn `IsClassOrChildClassFromArray`
  (params (Actor :type "Actor Object Reference") (Classes :type "Array of Actor Class Reference"))
  (returns (Valid :type Boolean))
  (locals (ClassFound :type Boolean))
  ;[1 1 1] Checks if the actor is of a specified type from a list (or child of a specified type).
  (for _array_element Classes
    (if (`self.IsClassOrChildClass` Actor _array_element)
      (set `local.ClassFound` true)
      (break)))
  (return (`local.ClassFound`)))

(fn `UpdateVisibilityInGame`
  ;[1 1 1] Update visibility
  (if (`self.VisibleInGame`)
    (`self.SetActorHiddenInGame` false)
    (else
      (`self.SetActorHiddenInGame` true))))

(fn `UserConstructionScript`
  ;[1 1 1] Set visibility and update the puzzle logic debug visualiser (showing connections between all puzzle logic actors).
  (`self.UpdateVisibilityInGame`)
  (bind _outactors (`GameplayStatics.GetAllActorsOfClass` "/Game/PuzzleLogicSystem/PLS_Blueprints/Misc/BP_PuzzleLogicVisualiser.BP_PuzzleLogicVisualiser_C"))
  (bind _output (`|GetArrayItem` _outactors))
  (`/Engine/EditorBlueprintResources/StandardMacros.IsValid` _output
    (:`Is Valid`
      (`/Game/PuzzleLogicSystem/PLS_Blueprints/Misc/BP_PuzzleLogicVisualiser.UpdateConnections` _output))))