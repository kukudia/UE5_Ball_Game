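; Scanning component that drives material parameter collections for a radial scan effect centered on the player.
; Scan and Scan1 animate Radius in MPC_Radius and MPC_Radius1, while Tick writes the pawn location to MPC_Radius.
; Custom timeline macros loop on zero-length Delays and can ignore time dilation.
; BeginPlay caches X-ray and outline post-process components and BP_Ball's spring arm, but the pulse and toggle logic is disconnected.
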(event `Scan`
  (bind _progress (`self.Timeline` 2.0 true)
    (:`Update`
      (`KismetMaterialLibrary.SetScalarParameterValue` "/Game/ScanningSystem/Materials/PulseEffect/MPC_Radius.MPC_Radius" "Radius" _progress))))

(event `Scan1`
  (bind _progress (`self.Timeline` 2.0 true)
    (:`Update`
      (`KismetMaterialLibrary.SetScalarParameterValue` "/Game/ScanningSystem/Materials/LandscapeScan/MPC_Radius1.MPC_Radius1" "Radius" _progress))))

(event `self.ReceiveBeginPlay`
  ;[0.07604 0.07604 0.07604] Sets components and gets
  (bind _returnvalue (`GameplayStatics.GetActorOfClass` "/Game/ScanningSystem/Materials/XRay/BP_PostProcess.BP_PostProcess_C"))
  (set `self.Xray` (`/Game/ScanningSystem/Materials/XRay/BP_PostProcess.PostProcess` _returnvalue))
  (bind _returnvalue_2 (`GameplayStatics.GetActorOfClass` "/Game/ScanningSystem/Materials/Outline/BP_OutlineFX.BP_OutlineFX_C"))
  (set `self.Outline` (`/Game/ScanningSystem/Materials/Outline/BP_OutlineFX.PostProcess` _returnvalue_2))
  ;[0.725 0.06948 0.04639] This part makes Focus effect. Replace actor class with your Character and set them again accordingly. If you want to have a sphere you must set it manually in a viewport
  (bind _returnvalue_3 (`GameplayStatics.GetActorOfClass` "/Game/01_Blueprints/BP_Ball.BP_Ball_C"))
  (set `self.Camera Boom_0` (`/Game/01_Blueprints/BP_Ball.SpringArm` _returnvalue_3)))

(event `self.ReceiveTick`
  (params (DeltaSeconds :type "Float (single-precision)"))
  (bind (_returnvalue_x _returnvalue_y _returnvalue_z) (`KismetMathLibrary.BreakVector` (`Actor.K2_GetActorLocation` (`GameplayStatics.GetPlayerPawn` 0))))
  ;[0.05521 0.05521 0.05521] Updates Character Location to generate effect from character origin
  (`KismetMaterialLibrary.SetVectorParameterValue` "/Game/ScanningSystem/Materials/PulseEffect/MPC_Radius.MPC_Radius" "Character Position" (make `LinearColor` _returnvalue_x _returnvalue_y _returnvalue_z 1.0)))

(event `Key|O`
  (params (Key :type "Key Structure"))
  ;[0.2469 0.1109 0.2115] Outline effect enable on O
)

(event `Key|L`
  (params (Key :type "Key Structure")))

(event `Key|R`
  (params (Key :type "Key Structure"))
  ;[0 0.02751 0.301] XRay effect enable on R
)

(event `Key|P`
  (params (Key :type "Key Structure"))
  ;[0.2385 0.236 0.07916] Pulse effect enable on P
)