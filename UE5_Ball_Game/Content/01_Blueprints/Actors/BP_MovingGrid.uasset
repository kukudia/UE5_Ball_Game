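; BP_MovingGrid is a puzzle-driven platform that moves a BP_MovingCollision child actor, with attached actors, along waypoints.
; Puzzle states start forward, reverse, flip-flop or indexed-waypoint moves, or pause it.
; Tick steps it using precomputed segment distances, per-waypoint waits and separate reverse speed, optionally holding position when a collision sweep is blocked.
; Arrivals at target waypoints pause the looping sound, play a stop sound and can trigger linked actors.
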(event `self.ReceiveBeginPlay`
  (bind _returnvalue (`KismetArrayLibrary.Array_Length` (`self.Waypoints`)))
  ;[1 1 1] Spawn looping moving sound effect.
  ; Pre-calculate and store the distances of each waypoint to the next.
  ; Set the platform at the desired starting waypoint location.
  ; Attach any actors (parented to this platform in the world outliner) to the moving platform child actor and set them to ignore collision to each other.
  (`parent.ReceiveBeginPlay`)
  (`|ExecutionSequence`
    (:`then_0`
      (`self.SpawnAndAttachSoundFX`)
      (for _index (range (+ (- _returnvalue 2) 1))
        (`KismetArrayLibrary.Array_Add` (`self.DistancesToNextWaypoint`) (`KismetMathLibrary.VSize` (- (`self.GetWaypointLocation` _index) (`self.GetWaypointLocation` (+ _index 1)))))))
    (:`then_1`
      (if (> _returnvalue 0)
        (`self.SetPlatformStartPos` (`self.StartingWaypoint`))
        (if (`self.AutoActivate`)
          (`self.StartMoveToTargetWaypoint` (- (`KismetArrayLibrary.Array_Length` (`self.Waypoints`)) 1)))))
    (:`then_2`
      (`/Game/PuzzleLogicSystem/PLS_Blueprints/Misc/BP_MovingCollision.AttachActorsAndIgnoreCollision` (`self.GetChildActorPlatform` (`self.ChildActor_MovingPlatform`)) (`self.GetAttachedActors` true)))
    (:`then_3`
      (if (== (`self.ReverseSpeed`) -1.0)
        (set `self.ReverseSpeed` (`self.MoveSpeed`))))))

(event `self.OnEnterState`
  (params (State :type "/Game/PuzzleLogicSystem/PLS_Blueprints/Misc/ENUM_LogicTriggerStates Enum" :default "NewEnumerator0"))
  (bind (_state1waypointindex _state2waypointindex _state3waypointindex _state4waypointindex _state5waypointindex) (break `/Game/PuzzleLogicSystem/PLS_Blueprints/Misc/STRUCT_MovingPlatformStates` (`self.StateWaypointIndices`)))
  ;[1 1 1] Puzzle logic event received to make the platform go forwards, backwards, or start moving to a specific waypoint.
  (`parent.OnEnterState` State)
  (switch `/Game/PuzzleLogicSystem/PLS_Blueprints/Misc/ENUM_LogicTriggerStates` State
    (:`NewEnumerator0`
      (`self.StartMoveToTargetWaypoint` (- (`KismetArrayLibrary.Array_Length` (`self.Waypoints`)) 1) :!label _label)
      (set `self.ActualSpeed` (`self.MoveSpeed`)))
    (:`NewEnumerator1`
      (`self.StartMoveToTargetWaypoint` 0 :!label _label_2)
      (set `self.ActualSpeed` (`self.ReverseSpeed`)))
    (:`NewEnumerator15`
      (if (`self.SettledAtStart`)
        (goto _label)
        (elif (`self.SettledAtEnd`)
          (goto _label_2)
          (elif (`self.IsMovingForward`)
            (goto _label_2)
            (else
              (goto _label))))))
    (:`NewEnumerator14`
      (set `self.Paused` true))
    (:`NewEnumerator2`
      (`self.StartMoveToTargetWaypoint` _state1waypointindex))
    (:`NewEnumerator3`
      (`self.StartMoveToTargetWaypoint` _state2waypointindex))
    (:`NewEnumerator4`
      (`self.StartMoveToTargetWaypoint` _state3waypointindex))
    (:`NewEnumerator5`
      (`self.StartMoveToTargetWaypoint` _state4waypointindex))
    (:`NewEnumerator6`
      (`self.StartMoveToTargetWaypoint` _state5waypointindex))))

(event `self.ReceiveTick`
  (params (DeltaSeconds :type "Float (single-precision)"))
  ;[1 1 1] Update platform position if it is moving.
  (`parent.ReceiveTick` DeltaSeconds)
  (if (and (`self.IsMoving`) (not (`self.Paused`)))
    (`self.UpdatePlatformPosition`))
  (if (> (`self.CurrentWaitTimer`) 0.0)
    (set `self.CurrentWaitTimer` (- (`self.CurrentWaitTimer`) (`GameplayStatics.GetWorldDeltaSeconds`)))))

(fn `GetChildActorPlatform`
  (params (ChildActor :type "ChildActorComponent Object Reference"))
  (returns (DoorActor :type "/Game/PuzzleLogicSystem/PLS_Blueprints/Misc/BP_MovingCollision Object Reference"))
  ;[1 1 1] Gets the actor "BP_MovingCollision" from the child actor.
  (bind _asbp_moving_collision (cast `/Game/PuzzleLogicSystem/PLS_Blueprints/Misc/BP_MovingCollision` (`ChildActorComponent.ChildActor` ChildActor))
    (:`then`
      (return _asbp_moving_collision))
    (:`CastFailed`
      (return null))))

(fn `GetWaypointLocation`
  (params (Index :type Integer))
  (returns (Location :type "Vector Structure"))
  ;[1 1 1] Gets the world location of a given waypoint.
  (return (`self.K2_GetActorLocation` (`.Waypoint_2_668CD4B149400217D97AE1B5E7C4E0C2` (break `/Game/PuzzleLogicSystem/PLS_Blueprints/Misc/STRUCT_MovingPlatformWaypoint` (`|GetArrayItem` (`self.Waypoints`) Index))))))

(fn `GetWaypointStopDuration`
  (params (Index :type Integer))
  (returns (Duration :type "Float (double-precision)"))
  ;[1 1 1] Gets the duration that the platform is set to wait for at a given waypoint, before it starts to move onto the next waypoint.
  (return (`.WaitTime_8_2FB870254620EB3ED300ECB303130A85` (break `/Game/PuzzleLogicSystem/PLS_Blueprints/Misc/STRUCT_MovingPlatformWaypoint` (`|GetArrayItem` (`self.Waypoints`) Index)))))

(fn `SetPlatformStartPos`
  (params (Index :type Integer))
  ;[1 1 1] Sets the platform to the selected starting waypoint's location.
  (bind _output_get (set `self.LastWaypoint` Index))
  (set `self.NextWaypoint` (+ _output_get 1))
  (set `self.TargetWaypoint` (- (`KismetArrayLibrary.Array_Length` (`self.Waypoints`)) 1))
  (`/Game/PuzzleLogicSystem/PLS_Blueprints/Misc/BP_MovingCollision.MC_SetWorldLocation` (`self.GetChildActorPlatform` (`self.ChildActor_MovingPlatform`)) (`self.GetWaypointLocation` Index) false)
  (set `self.DistanceRemainingToNextWaypoint` (`|GetArrayItem` (`self.DistancesToNextWaypoint`) (`self.LastWaypoint`))))

(fn `SpawnAndAttachSoundFX`
  ;[1 1 1] Creates a looping sound effect and sets it to paused on creation.
  ; This sound effect is turned on and off as the platform moves and stops.
  (bind _returnvalue (`GameplayStatics.SpawnSoundAttached` (`self.MovingLoopSFX`) (`self.ChildActor_MovingPlatform`) "None" (0.0 0.0 0.0) (struct) "SnapToTarget" true 1.0 1.0 0.0 "/Game/PuzzleLogicSystem/FX_Sound/Attenuation_MovingPlatform.Attenuation_MovingPlatform" null))
  (bind _output_get (set `self.AttachedSound` _returnvalue))
  (`AudioComponent.SetPaused` _output_get true))

(fn `StartMoveToTargetWaypoint`
  (params (WaypointIndex :type Integer))
  (bind _returnvalue (`KismetArrayLibrary.Array_Length` (`self.Waypoints`)))
  ;[1 1 1] Sets the platform to start moving to the target waypoint.
  ; This function performs logic to determine whether the platform needs to move forward or backward to reach the desired waypoint.
  (if (> _returnvalue 0)
    (if (< WaypointIndex _returnvalue)
      (if (not (or (and (== WaypointIndex 0) (`self.SettledAtStart`)) (and (== WaypointIndex (- _returnvalue 1)) (`self.SettledAtEnd`))))
        (set `self.IsMoving` true)
        (`AudioComponent.SetPaused` (`self.AttachedSound`) false)
        (set `self.Paused` false)
        (set `self.TargetWaypoint` WaypointIndex)
        (if (and (`self.IsMovingForward`) (<= (`self.TargetWaypoint`) (`self.LastWaypoint`)))
          (set `self.IsMovingForward` false)
          (set `self.DistanceRemainingToNextWaypoint` (- (`|GetArrayItem` (`self.DistancesToNextWaypoint`) (- (`self.NextWaypoint`) 1)) (`self.DistanceRemainingToNextWaypoint`)))
          (bind _output_get (set `self.NextWaypoint` (`self.LastWaypoint`)))
          (set `self.LastWaypoint` (+ _output_get 1))
          (set `self.ActualSpeed` (`self.ReverseSpeed`) :!label _label)
          (else
            (if (and (not (`self.IsMovingForward`)) (>= (`self.TargetWaypoint`) (`self.LastWaypoint`)))
              (set `self.IsMovingForward` true)
              (set `self.DistanceRemainingToNextWaypoint` (- (`|GetArrayItem` (`self.DistancesToNextWaypoint`) (`self.NextWaypoint`)) (`self.DistanceRemainingToNextWaypoint`)))
              (bind _output_get_2 (set `self.LastWaypoint` (`self.NextWaypoint`)))
              (bind _output_get_3 (set `self.NextWaypoint` (+ _output_get_2 1)))
              (set `self.NextWaypoint` _output_get_3)
              (elif (`self.IsMovingForward`)
                _
                (else
                  (goto _label))))
            (set `self.ActualSpeed` (`self.MoveSpeed`)))))
      (else
        (`KismetSystemLibrary.PrintString` "Attempting to move to invalid waypoint index")))
    (else
      (`KismetSystemLibrary.PrintString` "Moving platform has 0 waypoints"))))

(fn `UpdatePlatformPosition`
  (locals (TargetPosition :type "Vector Structure") (AmountToMove :type "Float (double-precision)") (ReachedWaypoint :type Boolean))
  (bind _distancestonextwaypoint (`self.DistancesToNextWaypoint`))
  (bind _targetwaypoint (`self.TargetWaypoint`))
  (bind _nextwaypoint (`self.NextWaypoint`))
  (bind _lastwaypoint (`self.LastWaypoint`))
  (bind (_state1waypointindex _state2waypointindex _state3waypointindex _state4waypointindex _state5waypointindex) (break `/Game/PuzzleLogicSystem/PLS_Blueprints/Misc/STRUCT_MovingPlatformStates` (`self.StateWaypointIndices`)))
  (bind _returnvalue (`KismetArrayLibrary.Array_Length` (`self.Waypoints`)))
  (bind _dooractor (`self.GetChildActorPlatform` (`self.ChildActor_MovingPlatform`)))
  (bind _returnvalue_2 (- _returnvalue 1))
  (bind _returnvalue_3 (- _returnvalue 2))
  ;[1 1 1] Logic to handle the platform moving from waypoint to the next.
  ; Also checks if the platform is being blocked by an object, and stops moving if true until blocker is gone.
  (if (not (> (`self.CurrentWaitTimer`) 0.0))
    (`|ExecutionSequence`
      (:`then_0`
        (bind _output_get (set `local.AmountToMove` (* (`GameplayStatics.GetWorldDeltaSeconds`) (`self.ActualSpeed`))))
        (if (>= _output_get (`self.DistanceRemainingToNextWaypoint`))
          (set `local.ReachedWaypoint` true)
          (set `local.AmountToMove` (`self.DistanceRemainingToNextWaypoint`))
          (set `self.CurrentWaitTimer` (`self.GetWaypointStopDuration` (`self.NextWaypoint`))))
        (`|ExecutionSequence`
          (:`then_0`
            (set `local.TargetPosition` (+ (`self.K2_GetActorLocation` (`self.GetChildActorPlatform` (`self.ChildActor_MovingPlatform`))) (* (`KismetMathLibrary.Normal` (- (`self.GetWaypointLocation` (`self.NextWaypoint`)) (`self.K2_GetActorLocation` (`self.GetChildActorPlatform` (`self.ChildActor_MovingPlatform`))))) (`local.AmountToMove`)))))
          (:`then_1`
            (if (`local.ReachedWaypoint`)
              (bind _isblocked (`/Game/PuzzleLogicSystem/PLS_Blueprints/Misc/BP_MovingCollision.MC_SetWorldLocation` _dooractor (`self.GetWaypointLocation` (`self.NextWaypoint`)) (`self.StopWhenBlocked`)))
              (if _isblocked
                (`/Game/PuzzleLogicSystem/PLS_Blueprints/Misc/BP_MovingCollision.MC_ResetToPreviousLocation` (`self.GetChildActorPlatform` (`self.ChildActor_MovingPlatform`)) :!label _label)
                (elif (== (`self.NextWaypoint`) (`self.TargetWaypoint`))
                  (set `self.IsMoving` false)
                  (`AudioComponent.SetPaused` (`self.AttachedSound`) true)
                  (`GameplayStatics.PlaySoundAtLocation` (`self.StopFX`) (`SceneComponent.K2_GetComponentLocation` (`self.ChildActor_MovingPlatform`)) (struct) 1.0 1.0 0.0 null null null null)
                  (if (== (`self.TargetWaypoint`) _returnvalue_2)
                    (set `self.TargetWaypoint` 0)
                    (set `self.LastWaypoint` _returnvalue_2)
                    (set `self.NextWaypoint` _returnvalue_3)
                    (set `self.DistanceRemainingToNextWaypoint` (`|GetArrayItem` (`self.DistancesToNextWaypoint`) _returnvalue_3))
                    ;[1 1 1] Trigger linked actors when the platform reaches the end (activate) or returns back to the start (deactivate).
                    ; Also handles looping behaviour if platform is set to do so.
                    (set `self.IsMovingForward` false)
                    (set `self.SettledAtEnd` true)
                    (`|ExecutionSequence`
                      (:`then_0`
                        (if (`self.Loop`)
                          (set `self.TargetWaypoint` (- (`KismetArrayLibrary.Array_Length` (`self.Waypoints`)) 1))
                          (set `self.LastWaypoint` 0)
                          (set `self.NextWaypoint` 1)
                          (set `self.DistanceRemainingToNextWaypoint` (`|GetArrayItem` (`self.DistancesToNextWaypoint`)))
                          (set `self.IsMovingForward` true)
                          (set `self.SettledAtStart` true)
                          (set `self.SettledAtEnd` false)))
                      (:`then_1`
                        (`self.TriggerLinkedActors` "NewEnumerator0")))
                    (elif (== (`self.TargetWaypoint`) 0)
                      (set `self.TargetWaypoint` _returnvalue_2)
                      (set `self.LastWaypoint` 0)
                      (set `self.NextWaypoint` 1)
                      (set `self.DistanceRemainingToNextWaypoint` (`|GetArrayItem` (`self.DistancesToNextWaypoint`)))
                      (set `self.IsMovingForward` true)
                      (set `self.SettledAtStart` true)
                      (`self.TriggerLinkedActors` "NewEnumerator1")
                      (else
                        ;[1 1 1] Trigger linked actors when the platform reaches a waypoint that's set up to do so.
                        (if (== _targetwaypoint _state1waypointindex)
                          (`self.TriggerLinkedActors` "NewEnumerator2")
                          (elif (== _targetwaypoint _state2waypointindex)
                            (`self.TriggerLinkedActors` "NewEnumerator3")
                            (elif (== _targetwaypoint _state3waypointindex)
                              (`self.TriggerLinkedActors` "NewEnumerator4")
                              (elif (== _targetwaypoint _state4waypointindex)
                                (`self.TriggerLinkedActors` "NewEnumerator5")
                                (elif (== _targetwaypoint _state5waypointindex)
                                  (`self.TriggerLinkedActors` "NewEnumerator6")))))))))
                  (elif (`self.IsMovingForward`)
                    (`/Engine/EditorBlueprintResources/StandardMacros.IncrementInt` _lastwaypoint
                      (:`  `
                        (`/Engine/EditorBlueprintResources/StandardMacros.IncrementInt` (`self.NextWaypoint`)
                          (:`  `
                            (set `self.DistanceRemainingToNextWaypoint` (`|GetArrayItem` _distancestonextwaypoint _lastwaypoint))))))
                    (else
                      (`/Engine/EditorBlueprintResources/StandardMacros.DecrementInt` (`self.LastWaypoint`)
                        (:`  `
                          (`/Engine/EditorBlueprintResources/StandardMacros.DecrementInt` _nextwaypoint
                            (:`  `
                              (set `self.DistanceRemainingToNextWaypoint` (`|GetArrayItem` _distancestonextwaypoint _nextwaypoint))))))))))
              (else
                (bind _isblocked_2 (`/Game/PuzzleLogicSystem/PLS_Blueprints/Misc/BP_MovingCollision.MC_SetWorldLocation` _dooractor (`local.TargetPosition`) (`self.StopWhenBlocked`)))
                (if _isblocked_2
                  (goto _label)
                  (else
                    (set `self.DistanceRemainingToNextWaypoint` (- (`self.DistanceRemainingToNextWaypoint`) (`local.AmountToMove`)))
                    (set `self.SettledAtEnd` false)
                    (set `self.SettledAtStart` false)))))))))))

(fn `UserConstructionScript`
  (`parent.UserConstructionScript`))