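; BP_Obstacle1 is an obstacle actor that slides along its Cube's forward vector by MoveDistance.
; On BeginPlay it caches start and end locations, sets the timeline play rate from MoveDuration and plays Timeline_Push from the start.
; Each update lerps the actor between the endpoints without sweep, with ResettingLocation selecting the direction.
; Finishing toggles that flag, but the graph does not replay the timeline.
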(event `self.ReceiveBeginPlay`
  (bind _returnvalue (`self.K2_GetActorLocation`))
  (set `self.StartLocation` _returnvalue)
  (set `self.EndLocation` (+ _returnvalue (* (`SceneComponent.GetForwardVector` (`self.Cube`)) (`self.MoveDistance`))))
  (`TimelineComponent.SetPlayRate` (`self.Timeline_Push`) (/ 1.0 (`self.MoveDuration`)))
  (bind (_direction _location) (`Timeline|Timeline_Push` :!via `PlayFromStart`)
    (:`Update`
      (`self.K2_SetActorLocation` (`KismetMathLibrary.VLerp` (`KismetMathLibrary.SelectVector` (`self.EndLocation`) (`self.StartLocation`) (`self.ResettingLocation`)) (`KismetMathLibrary.SelectVector` (`self.StartLocation`) (`self.EndLocation`) (`self.ResettingLocation`)) _location)))
    (:`Finished`
      (if (`self.ResettingLocation`)
        (set `self.ResettingLocation` false)
        (else
          (set `self.ResettingLocation` true))))))

(fn `UserConstructionScript`)