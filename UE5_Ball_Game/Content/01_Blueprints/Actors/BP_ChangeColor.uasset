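; BP_ChangeColor is a colored station that changes a BP_Ball's color, provided the ball currently has the required color.
; Box overlap stores itself on the ball and shows an interact prompt if CheckValid passes; leaving hides the prompt but keeps the reference.
; ChangeColor, not called here, rechecks validity, then swaps the ball's color and material with a sound, or plays an invalid sound.
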(event `self.ReceiveBeginPlay`
  (`self.AttemptWidget`)
  (`self.InitializeMaterial`))

(event `self.Box.OnComponentBeginOverlap`
  (params (OverlappedComponent :type "PrimitiveComponent Object Reference") (OtherActor :type "Actor Object Reference") (OtherComp :type "PrimitiveComponent Object Reference") (OtherBodyIndex :type Integer) (bFromSweep :type Boolean) (SweepResult :type "HitResult Structure (by ref)"))
  (bind _asbp_ball (cast `/Game/01_Blueprints/BP_Ball` OtherActor))
  (set `/Game/01_Blueprints/BP_Ball.ChangeColorActor` self _asbp_ball)
  (`self.CheckValid` _asbp_ball))

(event `self.Box.OnComponentEndOverlap`
  (params (OverlappedComponent :type "PrimitiveComponent Object Reference") (OtherActor :type "Actor Object Reference") (OtherComp :type "PrimitiveComponent Object Reference") (OtherBodyIndex :type Integer))
  (bind _asbp_ball (cast `/Game/01_Blueprints/BP_Ball` OtherActor))
  (set `/Game/01_Blueprints/BP_Ball.ChangeColorActor` self _asbp_ball)
  (`Widget.SetVisibility` (`self.WidgetInteractPrompt`) "Hidden"))

(fn `AttemptWidget`
  (bind _returnvalue (`PlayerController.GetHUD` (`GameplayStatics.GetPlayerController` 0)))
  ;[1 1 1] Attempt to add the interact widget prompt to the screen.
  (`/Engine/EditorBlueprintResources/StandardMacros.IsValid` _returnvalue
    (:`Is Valid`
      (bind _returnvalue_2 (`AddComponent|NODE_AddWidgetComponent-1` :`self` _returnvalue))
      (bind _returnvalue_3 (`|CreateWidget` "/Game/01_Blueprints/Widget_Interact.Widget_Interact_C" (`GameplayStatics.GetPlayerController` 0)))
      (bind _output_get (set `self.WidgetInteractPrompt` _returnvalue_3))
      (`WidgetComponent.SetWidget` _returnvalue_2 _output_get)
      (`UserWidget.AddToPlayerScreen` _returnvalue_3 0)
      (`WidgetComponent.SetWidgetSpace` _returnvalue_2 "Screen")
      (`Widget.SetVisibility` (`self.WidgetInteractPrompt`) "Hidden"))
    (:`Is Not Valid`
      ;[1 1 1] Add widget directly to screen if there is no HUD
      (bind _returnvalue_4 (`|CreateWidget` "/Game/01_Blueprints/Widget_Interact.Widget_Interact_C" (`GameplayStatics.GetPlayerController` 0)))
      (bind _output_get_2 (set `self.WidgetInteractPrompt` _returnvalue_4))
      (`UserWidget.AddToViewport` _output_get_2 0))))

(fn `ChangeColor`
  (params (BP_Ball :type "/Game/01_Blueprints/BP_Ball Object Reference"))
  (bind _ball (`/Game/01_Blueprints/BP_Ball.Ball` BP_Ball))
  (bind _isvalid (`self.CheckValid` BP_Ball))
  (if _isvalid
    (`GameplayStatics.PlaySound2D` "/Game/00_Imports/Audio/ChangeColor.ChangeColor" 1.0 1.0 0.0 null null)
    (bind _output_get (set `/Game/01_Blueprints/BP_Ball.CurrentColor` (`self.Color`) BP_Ball))
    (switch `/Game/01_Blueprints/Enums/Enum_PlayerState` _output_get
      (:`NewEnumerator0`
        (`PrimitiveComponent.SetMaterial` _ball 0 "/Game/03_Materials/M_FluorescentRed.M_FluorescentRed"))
      (:`NewEnumerator1`
        (`PrimitiveComponent.SetMaterial` _ball 0 "/Game/03_Materials/M_FluorescentGreen.M_FluorescentGreen"))
      (:`NewEnumerator2`
        (`PrimitiveComponent.SetMaterial` _ball 0 "/Game/03_Materials/M_FluorescentBlue.M_FluorescentBlue")))
    (`self.CheckValid` BP_Ball)
    (else
      (`GameplayStatics.PlaySound2D` "/Game/00_Imports/Audio/Invalid.Invalid" 1.0 1.0 0.0 null null))))

(fn `CheckValid`
  (params (BP_Ball :type "/Game/01_Blueprints/BP_Ball Object Reference"))
  (returns (isValid :type Boolean))
  (bind _widgetinteractprompt (`self.WidgetInteractPrompt`))
  (if (== (`KismetMathLibrary.Conv_ByteToInt` (`/Game/01_Blueprints/BP_Ball.CurrentColor` BP_Ball)) (`KismetMathLibrary.Conv_ByteToInt` (`self.Required State`)))
    (`Widget.SetVisibility` _widgetinteractprompt "Visible")
    (return true)
    (else
      (`Widget.SetVisibility` _widgetinteractprompt "Hidden")
      (return false))))

(fn `InitializeMaterial`
  (bind _cube (`self.Cube`))
  (switch `/Game/01_Blueprints/Enums/Enum_PlayerState` (`self.Color`)
    (:`NewEnumerator0`
      (`PrimitiveComponent.SetMaterial` _cube 0 "/Game/03_Materials/M_FluorescentRed.M_FluorescentRed"))
    (:`NewEnumerator1`
      (`PrimitiveComponent.SetMaterial` _cube 0 "/Game/03_Materials/M_FluorescentGreen.M_FluorescentGreen"))
    (:`NewEnumerator2`
      (`PrimitiveComponent.SetMaterial` _cube 0 "/Game/03_Materials/M_FluorescentBlue.M_FluorescentBlue"))))

(fn `UserConstructionScript`)