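; BP_MoveUpObject1 is an actor that moves along its Cube's up vector by MoveDistance.
; A timeline started on BeginPlay, rate-scaled by MoveDuration, lerps the location between start and end points.
; On finish it flips ResettingLocation, which swaps the lerp direction, but nothing here replays the timeline.
; Tick captures both endpoints once via SetLocation and draws a debug line between them every frame.
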(event `self.ReceiveBeginPlay`
  (`TimelineComponent.SetPlayRate` (`self.Timeline_Push`) (/ 1.0 (`self.MoveDuration`)))
  (bind (_direction _location) (`Timeline|Timeline_Push`)
    (:`Update`
      (`self.K2_SetActorLocation` (`KismetMathLibrary.VLerp` (`KismetMathLibrary.SelectVector` (`self.EndLocation`) (`self.StartLocation`) (`self.ResettingLocation`)) (`KismetMathLibrary.SelectVector` (`self.StartLocation`) (`self.EndLocation`) (`self.ResettingLocation`)) _location)))
    (:`Finished`
      (if (`self.ResettingLocation`)
        (set `self.ResettingLocation` false)
        (else
          (set `self.ResettingLocation` true))))))

(event `self.ReceiveTick`
  (params (DeltaSeconds :type "Float (single-precision)"))
  (`self.SetLocation`)
  (`KismetSystemLibrary.DrawDebugLine` (`self.StartLocation`) (`self.EndLocation`) (struct :`R` 1.0 :`G` 0.999691 :`A` 1.0) 0.0 0.1))

(fn `SetLocation`
  (bind _returnvalue (`self.K2_GetActorLocation`))
  (if (not (`self.IsSetLocation`))
    (set `self.StartLocation` _returnvalue)
    (set `self.EndLocation` (+ _returnvalue (* (`SceneComponent.GetUpVector` (`self.Cube`)) (`self.MoveDistance`))))
    (set `self.IsSetLocation` true)))

(fn `UserConstructionScript`)