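; BP_Grid is a puzzle-linked grid actor that acts as a door, sliding open and closed.
; On BeginPlay it initializes its ComponentPuzzleOwner with a PuzzleId.
; OpenDoor and CloseDoor forward to Open and Close, which play or reverse one timeline that lerps the Grid's relative location between start and end positions without sweeping.
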(event `self.ReceiveBeginPlay`
  (`/Game/01_Blueprints/Components/Component_PuzzleOwner.Initialize` (`self.Component_PuzzleOwner`) (`self.PuzzleId`)))

(event `Open`
  (bind (_direction _opendoor) (`Timeline|Timeline_Open` :!label _label)
    (:`Update`
      (`SceneComponent.K2_SetRelativeLocation` (`self.Grid`) (`KismetMathLibrary.VLerp` (`self.StartLocation`) (`self.EndLocation`) _opendoor) false false))))

(event `Close`
  (goto _label :!via `Reverse`))

(event `self.OpenDoor`
  (`self.Open`))

(event `Event CloseDoor`
  (`self.Close`))

(fn `UserConstructionScript`)